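; BP_Scientist is the player's 2D sprite character, with Enhanced Input movement, jump, crouch and an airborne dive.
; Landing from a dive notifies hit actors implementing BPI_Diveable.
; Tick flips the sprite by velocity and picks idle, walk or crouch flipbooks.
; It also creates the health bar, toggles a pausing menu on Escape, and adjusts health with O/P keys, printing a death message when low.
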(event `Key|O`
  (params (Key :type "Key Structure"))
  (bind _returnvalue (`KismetMathLibrary.FClamp` (- (`self.Vie`) 5.0) 0.0 100.0))
  (:`Pressed`
    (if (<= _returnvalue 10.0)
      (`KismetSystemLibrary.PrintString` "Vous etes mort !!!")
      (else
        (set `self.Vie` _returnvalue)))))

(event `Key|P`
  (params (Key :type "Key Structure"))
  (:`Pressed`
    (set `self.Vie` (`KismetMathLibrary.FClamp` (+ (`self.Vie`) 5.0) 0.0 100.0))))

(event `self.ReceiveBeginPlay`
  (`|ExecutionSequence`
    (:`then_0`
      ;[1 1 1] Défini la conf des touches par défaut
      (`EnhancedInputSubsystemInterface.AddMappingContext` (pcsubsystem `EnhancedInputLocalPlayerSubsystem` (`GameplayStatics.GetPlayerController` 0)) "/Game/TheMadScientist/Core/Inputs/IMC_Default.IMC_Default" 0 (struct)))
    (:`then_1`
      (bind _returnvalue (`|CreateWidget` "/Game/TheMadScientist/Interface/BarreVie/Barre_Vie.Barre_Vie_C"))
      (`UserWidget.AddToViewport` _returnvalue 0))))

(event `EnhancedInput|/Game/TheMadScientist/Core/Inputs/INP_MoveAround`
  (params (ActionValue :type "Float (double-precision)") (ElapsedSeconds :type "Float (double-precision)") (TriggeredSeconds :type "Float (double-precision)") (InputAction :type "InputAction Object Reference" :default "/Game/TheMadScientist/Core/Inputs/INP_MoveAround.INP_MoveAround"))
  ;[1 1 1] Déplacements
  (:`Triggered`
    (`self.AddMovementInput` (`self.GetActorForwardVector`) ActionValue)))

(event `EnhancedInput|/Game/TheMadScientist/Core/Inputs/INP_Jump`
  (params (ActionValue :type Boolean) (ElapsedSeconds :type "Float (double-precision)") (TriggeredSeconds :type "Float (double-precision)") (InputAction :type "InputAction Object Reference" :default "/Game/TheMadScientist/Core/Inputs/INP_Jump.INP_Jump"))
  (bind _charactermovement (`self.CharacterMovement`))
  (:`Started`
    (`self.Jump`)
    (if (`KismetMathLibrary.BooleanNOR` (`NavMovementComponent.IsFalling` _charactermovement) (`NavMovementComponent.IsCrouching` _charactermovement))
      (`GameplayStatics.SpawnSound2D` "/Game/TheMadScientist/Audio/A_Powerup.A_Powerup" 0.3 1.0 0.0 null)))
  (:`Completed`
    (`self.StopJumping`)))

(event `EnhancedInput|/Game/TheMadScientist/Core/Inputs/INP_Crouch`
  (params (ActionValue :type Boolean) (ElapsedSeconds :type "Float (double-precision)") (TriggeredSeconds :type "Float (double-precision)") (InputAction :type "InputAction Object Reference" :default "/Game/TheMadScientist/Core/Inputs/INP_Crouch.INP_Crouch"))
  (bind _sprite (`self.Sprite`))
  (:`Started`
    (if (`NavMovementComponent.IsFalling` (`self.CharacterMovement`))
      (set `self.diving` (not (`self.diving`)))
      (`self.LaunchCharacter` (0.0 0.0 -1500.0))
      (else
        (`self.Crouch`)
        (`SceneComponent.K2_SetRelativeLocation` _sprite (0.0 0.0 -43.0) false true))))
  (:`Completed`
    (`self.UnCrouch`)
    (`SceneComponent.K2_SetRelativeLocation` _sprite (0.0 0.0 -43.0) false false)))

(event `self.OnLanded`
  (params (Hit :type "HitResult Structure (by ref)"))
  (bind (_bblockinghit _binitialoverlap _time _distance _location _impactpoint _normal _impactnormal _physmat _hitactor) (`GameplayStatics.BreakHitResult` Hit))
  (`|ExecutionSequence`
    (:`then_0`
      (if (and (`KismetSystemLibrary.DoesImplementInterface` _hitactor "/Game/TheMadScientist/Core/BPI_Diveable.BPI_Diveable_C") (`self.diving`))
        (message `/Game/TheMadScientist/Core/BPI_Diveable.OnHitByDive` _hitactor)))
    (:`then_1`
      (set `self.diving` false))))

(event `self.ReceiveTick`
  (params (DeltaSeconds :type "Float (single-precision)"))
  (bind _sprite (`self.Sprite`))
  (bind _returnvalue (`NavMovementComponent.IsCrouching` (`self.CharacterMovement`)))
  (`|ExecutionSequence`
    (:`then_0`
      (`/Engine/EditorBlueprintResources/StandardMacros.CompareFloat` (`KismetMathLibrary.Dot_VectorVector` (`KismetMathLibrary.Normal` (`self.GetVelocity`)) (`KismetMathLibrary.GetForwardVector` (struct)))
        (:`>`
          (`SceneComponent.K2_SetRelativeRotation` :`self` _sprite))
        (:`<`
          (`SceneComponent.K2_SetRelativeRotation` _sprite (struct :`Yaw` 180.0) false false))))
    (:`then_1`
      (if (> (`KismetMathLibrary.VSizeXYSquared` (`CharacterMovementComponent.GetCurrentAcceleration` (`self.CharacterMovement`))) 0.0)
        (`PaperFlipbookComponent.SetFlipbook` (`self.Sprite`) (select `bool` _returnvalue :`false` "/Game/TheMadScientist/Art/Character/PFB_Walk.PFB_Walk" :`true` "/Game/TheMadScientist/Art/Character/PFB_CrouchWalk.PFB_CrouchWalk" :!type "PaperFlipbook Object Reference"))
        (else
          (`PaperFlipbookComponent.SetFlipbook` (`self.Sprite`) (select `bool` _returnvalue :`false` "/Game/TheMadScientist/Art/Character/PFB_Idle.PFB_Idle" :`true` "/Game/TheMadScientist/Art/Character/PFB_CrouchIdle.PFB_CrouchIdle" :!type "PaperFlipbook Object Reference")))))))

(event `EnhancedInput|/Game/TheMadScientist/Core/Inputs/Escape`
  (params (ActionValue :type Boolean) (ElapsedSeconds :type "Float (double-precision)") (TriggeredSeconds :type "Float (double-precision)") (InputAction :type "InputAction Object Reference" :default "/Game/TheMadScientist/Core/Inputs/Escape.Escape"))
  (bind _returnvalue (`GameplayStatics.GetPlayerController` 0))
  (:`Started`
    (if (not (`self.Ismainmenuopen`))
      (set `self.Ismainmenuopen` true)
      (bind _returnvalue_2 (`|CreateWidget` "/Game/TheMadScientist/Interface/MainMenu/MainMenu.MainMenu_C" _returnvalue))
      (bind _output_get (set `self.Pausemenu` _returnvalue_2))
      (`UserWidget.AddToViewport` _output_get 0)
      (`WidgetBlueprintLibrary.SetInputMode_GameAndUIEx` _returnvalue (`self.Pausemenu`))
      (set `PlayerController.bShowMouseCursor` true (`GameplayStatics.GetPlayerController` 0))
      (`GameplayStatics.SetGamePaused` true)
      (else
        (set `self.Ismainmenuopen` false)
        (`Widget.RemoveFromParent` (`self.Pausemenu`))
        (`GameplayStatics.SetGamePaused` false)
        (`WidgetBlueprintLibrary.SetInputMode_GameOnly` _returnvalue)
        (set `PlayerController.bShowMouseCursor` false (`GameplayStatics.GetPlayerController` 0))))))

(fn `UserConstructionScript`)